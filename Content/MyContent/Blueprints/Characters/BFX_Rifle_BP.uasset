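; Player weapon Blueprint owned by MyPlayerCharacter, handling rifle, pistol, high-powered rifle, thrown grenades and a grenade launcher.
; Trigger input runs through a gated fire-rate limiter, then line-traces camera aim and sphere-traces to threaten the owner and report AI damage events.
; Shots spawn projectiles, montages and FX, using selectable timeline camera or random cone recoil.
; It also manages noise reporting, muzzle smoke, aiming, zoom and bullet time.
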(event Custom|ClientStartNoise
  (Variables|Default|SetIsNoisy? true)
  (Class|AISenseHearing|ReportNoiseEvent (Transformation|GetActorLocation) 1.0 self 0.0 "Noise")
  (Utilities|FlowControl|Delay 2.0))

(event Custom|StartNoise
  (Networking|SwitchHasAuthority
    (:Authority
      (CallFunction|ClientStartNoise))))

(event Custom|ClientStopNoise
  (Variables|Default|SetIsNoisy? false))

(event Custom|StopNoise
  (Networking|SwitchHasAuthority
    (:Authority
      (CallFunction|ClientStopNoise))))

(event EventBeginPlay
  ;[1 1 1] BeginPlay
  ;;[1 1 1] Set GunOwner and Decal FadeScreenSize
  (bind _asmy_player_character (Utilities|Casting|CastToMyPlayerCharacter (Components|GetOwner)))
  (Variables|MyCharacter|SetGunOwner _asmy_player_character)
  (Development|ExecuteConsoleCommand (Utilities|String|Append "r.Decal.FadeScreenSizeMult " (Utilities|String|ToString(Float) (Variables|MyCharacter|GetDecal%20Fade%20Size%20Multiplier))) 0))

(event EventTick
  (params (DeltaSeconds :type Float%20%28single-precision%29))
  ;[1 1 1] Event tick - Movement and muzzle checks
  ;;[1 1 1] Movement Check
  (if (>= (Math|Vector|VectorLength (Variables|/Script/Engine.MovementComponent|GetVelocity (Variables|/Script/Engine.Character|GetCharacterMovement (Variables|MyCharacter|GetGunOwner)))) 8e+02)
    (Variables|MyCharacter|SetCharacterMoving true)
    ;;[0.2075 0.4327 1] Deactivate Muzzle Smoke On Movement Threshold
    (if (Components|Activation|IsActive (Variables|Default|GetMuzzle_Smoke_light)) :!label _label
      (CallFunction|MuzzleSmokeOff))
    (else
      (Variables|MyCharacter|SetCharacterMoving false)
      (if (Variables|MyCharacter|GetTriggerPressed)
        (goto _label)))))

(fn ConstructionScript)

(fn ThreatTrace
  (params (ThreatValue :type Float%20%28single-precision%29))
  (bind _arrow_bulletspawn (Variables|Default|GetArrow_BulletSpawn))
  (bind _returnvalue (Transformation|GetWorldLocation _arrow_bulletspawn))
  (bind _outhit (Collision|SphereTraceByChannel _returnvalue (+ _returnvalue (* (Math|Vector|GetForwardVector (Transformation|GetWorldRotation (Variables|/Game/MyContent/Blueprints/Characters/MyPlayerCharacter.MyPlayerCharacter_C|GetFollowCamera (Variables|MyCharacter|GetGunOwner)))) (Variables|Default|GetThreatRange))) ThreatValue "TraceTypeQuery2" false (Utilities|Array|MakeArray (Variables|MyCharacter|GetGunOwner)) "ForDuration" true "(R=0.088497,G=1.000000,B=0.693293,A=1.000000)" "(R=0.123496,G=0.042250,B=1.000000,A=1.000000)"))
  (if (.bblockinghit _outhit)
    (Utilities|Casting|CastToMyPlayerCharacter (.hitactor _outhit)
      (:then
        (Default|Threatened (Variables|MyCharacter|GetGunOwner)))
      (:CastFailed
        (bind _asenemy_npc (Utilities|Casting|CastToEnemyNPC (.hitactor _outhit)))
        (Default|Threatened (Variables|MyCharacter|GetGunOwner))
        (Class|AISenseDamage|ReportDamageEvent _asenemy_npc self 1e+01 (Transformation|GetActorLocation) (.impactpoint _outhit) "Damage")))))

(event Custom|TriggerPressedEvent
  (bind (_aimtransform_location _returnvalue) (|ConeRecoilWorkout_3_2))
  (bind (_aimtransform_location_2 _returnvalue_2) (|ConeRecoilWorkout_3))
  (bind (_aimtransform_location_3 _returnvalue_3) (|ConeRecoilWorkout))
  (bind (_aimtransform_location_4 _returnvalue_4) (|ConeRecoilWorkout_2))
  (bind _gunowner (Variables|MyCharacter|GetGunOwner))
  (bind _aimtransform (Variables|AimOffset|GetAimTransform))
  (bind _gunowner_2 (Variables|MyCharacter|GetGunOwner))
  (bind _recoiltype (Variables|RecoilOptions|GetRecoilType))
  (bind _gunowner_3 (Variables|MyCharacter|GetGunOwner))
  (bind _gunowner_4 (Variables|MyCharacter|GetGunOwner))
  (bind _gunowner_5 (Variables|MyCharacter|GetGunOwner))
  (bind _recoiltype_2 (Variables|RecoilOptions|GetRecoilType))
  (bind _aimtransform_2 (Variables|AimOffset|GetAimTransform))
  (bind _recoiltype_3 (Variables|RecoilOptions|GetRecoilType))
  (bind _aimtransform_3 (Variables|AimOffset|GetAimTransform))
  (bind _recoiltype_4 (Variables|RecoilOptions|GetRecoilType))
  (bind _aimtransform_4 (Variables|AimOffset|GetAimTransform))
  (bind _gunowner_6 (Variables|MyCharacter|GetGunOwner))
  (bind _returnvalue_5 (Utilities|Select :Index _recoiltype_2 :NewEnumerator0 _aimtransform_4 :NewEnumerator1 _aimtransform_4 :NewEnumerator2 (Math|Transform|MakeTransform _aimtransform_location _returnvalue "1,1,1")))
  (bind _returnvalue_6 (Utilities|Select :Index _recoiltype_3 :NewEnumerator0 _aimtransform_2 :NewEnumerator1 _aimtransform_2 :NewEnumerator2 (Math|Transform|MakeTransform _aimtransform_location_3 _returnvalue_3 "1,1,1")))
  (bind _returnvalue_7 (Utilities|Select :Index _recoiltype :NewEnumerator0 _aimtransform :NewEnumerator1 _aimtransform :NewEnumerator2 (Math|Transform|MakeTransform _aimtransform_location_2 _returnvalue_2 "1,1,1")))
  (bind _returnvalue_8 (Utilities|Select :Index _recoiltype_4 :NewEnumerator0 _aimtransform_3 :NewEnumerator1 _aimtransform_3 :NewEnumerator2 (Math|Transform|MakeTransform _aimtransform_location_4 _returnvalue_4 "1,1,1")))
  (bind _mesh (Variables|/Script/Engine.Character|GetMesh _gunowner))
  (bind _mesh_2 (Variables|/Script/Engine.Character|GetMesh _gunowner_3))
  (bind _mesh_3 (Variables|/Script/Engine.Character|GetMesh _gunowner_4))
  (bind _returnvalue_9 (Components|SkeletalMesh|GetAnimInstance _mesh))
  (bind _returnvalue_10 (Components|SkeletalMesh|GetAnimInstance _mesh_2))
  (bind _returnvalue_11 (Components|SkeletalMesh|GetAnimInstance _mesh_3))
  ;[1 1 1] Trigger Press
  (Variables|MyCharacter|SetTriggerPressed true)
  (if (Variables|MyCharacter|GetGunAudioToggle)
    (CallFunction|StartNoise))
  (|FireRateAndSpamClickRegulation (Utilities|Select :Index (Variables|MyCharacter|GetSelectedWeapon) :Option%200 (Variables|FireRate|GetRifle%20Fire%20Rate) :Option%201 (Variables|FireRate|GetPistol%20Fire%20Rate) :Option%202 (Variables|FireRate|GetHiPowered%20Fire%20Rate) :Option%203 (Variables|FireRate|GetThrowGrenadeRate))
    (:FireProjectile
      (CallFunction|MuzzleSmokeOff)
      (CallFunction|AimOffsetTrigger)
      (CallFunction|ThreatTrace 25.0)
      (switch int (Variables|MyCharacter|GetSelectedWeapon)
        (:0
          ;[1 1 1] Spawn Rifle projectile
          (if (Variables|MyCharacter|GetAiming)
            (Animation|Montage|MontagePlay _returnvalue_10 "/Game/MyContent/Animations/Rifle/Aim/Rifle_ShootBurstLong_Montage.Rifle_ShootBurstLong_Montage" 1.0 "MontageLength" 0.0 true)
            (else
              (Animation|Montage|MontagePlay _returnvalue_10 "/Game/MyContent/Animations/Rifle/Hip/Fire_Rifle_Hip_Montage.Fire_Rifle_Hip_Montage" 1.0 "MontageLength" 0.0 true)))
          (Game|SpawnActorfromClass "/Game/BallisticsVFX/FXSpawnerBlueprints/Projectiles/CubitUniProjectile.CubitUniProjectile_C" (Math|Transform|MakeTransform (.location _returnvalue_6) (.rotation _returnvalue_6) "1,1,1") "AlwaysSpawn" 0 3e+04 true true false "NewEnumerator1" 0 "NewEnumerator0" 0) ; Spawn projectile
          (if (Variables|MyCharacter|GetGunAudioToggle)
            (Audio|SpawnSoundAttached "/Game/BallisticsVFX/SFX/Guns/Rifle_fire.Rifle_fire" (Variables|Default|GetProjectileSpawnPoint) "None" "0, 0, 0" "0, 0, 0" "KeepRelativeOffset" false 1.0 (Class|GameplayStatics|GetGlobalTimeDilation) 0.0 0 0))
          ;[1 1 1] Muzzle Flash
          (Effects|SpawnEmitterAttached "/Game/BallisticsVFX/Particles/Muzzle/MuzzleFlash/Muzzle_Flash_Med.Muzzle_Flash_Med" (Variables|Default|GetProjectileSpawnPoint) "None" (Transformation|GetSocketLocation (Variables|Default|GetProjectileSpawnPoint) "None") (Math|Rotator|CombineRotators (Pawn|GetControlRotation (Variables|MyCharacter|GetGunOwner) :!class /Script/Engine.Pawn) "0, 0, 0") "1.000000,1.000000,1.000000" "KeepWorldPosition")
          ;[1 1 1] Shell and Ejector Port Smoke
          (Effects|SpawnEmitteratLocation "/Game/BallisticsVFX/Particles/BulletCasings/Bullet_Casing_2.Bullet_Casing_2" (Transformation|GetSocketLocation (Variables|Default|GetEjectorPort) "None") (Math|Rotator|CombineRotators (Pawn|GetControlRotation (Variables|MyCharacter|GetGunOwner) :!class /Script/Engine.Pawn) "0,90.000000, 0"))
          (switch Utilities|FlowControl|Switch|SwitchonRecoilType (Variables|RecoilOptions|GetRecoilType)
            (:NewEnumerator1
              ;[1 1 1] Recoil Rifle Fire
              (bind _recoil_float (Timeline|Timeline_0 PlayFromStart)
                (:Update
                  (Pawn|Input|AddControllerPitchInput _gunowner_5 (* (* (* _recoil_float (Variables|CameraRecoil|GetRifle_Recoil%20Amp)) (Math|Random|RandomFloatinRange 0.9 1.1)) (Variables|MyCharacter|GetBaseLookUpRate) (Utilities|Time|GetWorldDeltaSeconds)))
                  (Pawn|Input|AddControllerYawInput _gunowner_5 (* (* (* (* (* _recoil_float (Variables|CameraRecoil|GetRifle_Recoil%20Amp)) (Math|Random|RandomFloatinRange 0.9 1.1)) (Variables|CameraRecoil|GetRifle_sideways)) (Math|Random|RandomFloatinRange -1.0 1.0)) (Variables|MyCharacter|GetBaseTurnRate) (Utilities|Time|GetWorldDeltaSeconds))))))
            (:NewEnumerator2
              (CallFunction|ConeRecoil))))
        (:1
          ;[1 1 1] Spawn Pistol projectile
          (if (Variables|MyCharacter|GetAiming)
            (Animation|Montage|MontagePlay _returnvalue_11 "/Game/MyContent/Animations/Pistol/IronSights/Pistol_ShootPowerful_Montage.Pistol_ShootPowerful_Montage" 1.0 "MontageLength" 0.0 true)
            (Utilities|FlowControl|Delay 0.1)
            (else
              (Animation|Montage|MontagePlay _returnvalue_11 "/Game/MyContent/Animations/Pistol/IronSights/Pistol_ShootOnce_Montage.Pistol_ShootOnce_Montage" 1.0 "MontageLength" 0.0 true)
              ;;[1 1 1] Wait until gun raised
              (Utilities|FlowControl|Delay 0.3)))
          (Game|SpawnActorfromClass "/Game/BallisticsVFX/FXSpawnerBlueprints/Projectiles/CubitUniProjectile.CubitUniProjectile_C" (Math|Transform|MakeTransform (.location _returnvalue_8) (.rotation _returnvalue_8) "1,1,1") "AlwaysSpawn" 0 1.5e+04 true true false "NewEnumerator1" 0 "NewEnumerator0" 0) ; Spawn projectile
          (if (Variables|MyCharacter|GetGunAudioToggle)
            (Audio|SpawnSoundAttached "/Game/BallisticsVFX/SFX/Guns/Pistol_fire.Pistol_fire" (Variables|Default|GetProjectileSpawnPoint) "None" "0, 0, 0" "0, 0, 0" "KeepRelativeOffset" false 1.0 (Class|GameplayStatics|GetGlobalTimeDilation) 0.0 0 0))
          ;[1 1 1] Muzzle Flash
          (Effects|SpawnEmitterAttached "/Game/BallisticsVFX/Particles/Muzzle/MuzzleFlash/Muzzle_Flash_Small.Muzzle_Flash_Small" (Variables|Default|GetProjectileSpawnPoint) "None" (Transformation|GetSocketLocation (Variables|Default|GetProjectileSpawnPoint) "None") (Math|Rotator|CombineRotators (Pawn|GetControlRotation (Variables|MyCharacter|GetGunOwner) :!class /Script/Engine.Pawn) "0, 0, 0") "1.000000,1.000000,1.000000" "KeepWorldPosition")
          ;[1 1 1] Shell and Ejector Port Smoke
          (Effects|SpawnEmitteratLocation "/Game/BallisticsVFX/Particles/BulletCasings/Bullet_Casing_2.Bullet_Casing_2" (Transformation|GetSocketLocation (Variables|Default|GetEjectorPort) "None") (Math|Rotator|CombineRotators (Pawn|GetControlRotation (Variables|MyCharacter|GetGunOwner) :!class /Script/Engine.Pawn) "0,90.000000, 0"))
          (switch Utilities|FlowControl|Switch|SwitchonRecoilType (Variables|RecoilOptions|GetRecoilType)
            (:NewEnumerator1
              ;[1 1 1] Recoil Pistol Fire
              (bind _recoil_float_2 (Timeline|Timeline_1 PlayFromStart)
                (:Update
                  (Pawn|Input|AddControllerPitchInput _gunowner_6 (* (* (* _recoil_float_2 (Variables|CameraRecoil|GetPistol_Recoil%20Amp)) (Math|Random|RandomFloatinRange 0.9 1.1)) (Variables|MyCharacter|GetBaseLookUpRate) (Utilities|Time|GetWorldDeltaSeconds)))
                  (Pawn|Input|AddControllerYawInput _gunowner_6 (* (* (* (* (* _recoil_float_2 (Variables|CameraRecoil|GetPistol_Recoil%20Amp)) (Math|Random|RandomFloatinRange 0.9 1.1)) (Variables|CameraRecoil|GetPistol_sideways)) (Math|Random|RandomFloatinRange -1.0 1.0)) (Variables|MyCharacter|GetBaseTurnRate) (Utilities|Time|GetWorldDeltaSeconds))))))
            (:NewEnumerator2
              (CallFunction|ConeRecoil))))
        (:2
          ;[1 1 1] Spawn HP Rifle projectile
          (if (Variables|MyCharacter|GetAiming)
            (Animation|Montage|MontagePlay _returnvalue_9 "/Game/MyContent/Animations/Rifle/Aim/Rifle_ShootBurst_Montage.Rifle_ShootBurst_Montage" 1.0 "MontageLength" 0.0 true)
            (else
              (Animation|Montage|MontagePlay _returnvalue_9 "/Game/MyContent/Animations/Rifle/Hip/Fire_Rifle_Hip_Montage.Fire_Rifle_Hip_Montage" 1.0 "MontageLength" 0.0 true)))
          (Game|SpawnActorfromClass "/Game/BallisticsVFX/FXSpawnerBlueprints/Projectiles/CubitUniProjectile.CubitUniProjectile_C" (Math|Transform|MakeTransform (.location _returnvalue_7) (.rotation _returnvalue_7) "1,1,1") "AlwaysSpawn" 0 4e+04 true true false "NewEnumerator2" 0 "NewEnumerator0" 0) ; Spawn projectile
          (if (Variables|MyCharacter|GetGunAudioToggle)
            (Audio|SpawnSoundAttached "/Game/BallisticsVFX/SFX/Guns/HiPowered.HiPowered" (Variables|Default|GetProjectileSpawnPoint) "None" "0, 0, 0" "0, 0, 0" "KeepRelativeOffset" false 1.0 (Class|GameplayStatics|GetGlobalTimeDilation) 0.0 0 0))
          ;[1 1 1] Muzzle Flash
          (Effects|SpawnEmitterAttached "/Game/BallisticsVFX/Particles/Muzzle/MuzzleFlash/Muzzle_Flash_Med.Muzzle_Flash_Med" (Variables|Default|GetProjectileSpawnPoint) "None" (Transformation|GetSocketLocation (Variables|Default|GetProjectileSpawnPoint) "None") (Math|Rotator|CombineRotators (Pawn|GetControlRotation (Variables|MyCharacter|GetGunOwner) :!class /Script/Engine.Pawn) "0, 0, 0") "1.000000,1.000000,1.000000" "KeepWorldPosition")
          ;[1 1 1] Shell and Ejector Port Smoke
          (Effects|SpawnEmitteratLocation "/Game/BallisticsVFX/Particles/BulletCasings/Bullet_Casing_2.Bullet_Casing_2" (Transformation|GetSocketLocation (Variables|Default|GetEjectorPort) "None") (Math|Rotator|CombineRotators (Pawn|GetControlRotation (Variables|MyCharacter|GetGunOwner) :!class /Script/Engine.Pawn) "0,90.000000, 0"))
          (switch Utilities|FlowControl|Switch|SwitchonRecoilType (Variables|RecoilOptions|GetRecoilType)
            (:NewEnumerator1
              ;[1 1 1] Recoil Hi Powered Fire
              (bind _recoil_float_3 (Timeline|Timeline_5 PlayFromStart)
                (:Update
                  (Pawn|Input|AddControllerPitchInput _gunowner_2 (* (* (* _recoil_float_3 (Variables|CameraRecoil|GetHP_Recoil%20Amp)) (Math|Random|RandomFloatinRange 0.9 1.1)) (Variables|MyCharacter|GetBaseLookUpRate) (Utilities|Time|GetWorldDeltaSeconds)))
                  (Pawn|Input|AddControllerYawInput _gunowner_2 (* (* (* (* (* _recoil_float_3 (Variables|CameraRecoil|GetHP_Recoil%20Amp)) (Math|Random|RandomFloatinRange 0.9 1.1)) (Variables|CameraRecoil|GetHP_sideways)) (Math|Random|RandomFloatinRange -0.5 0.5)) (Variables|MyCharacter|GetBaseTurnRate) (Utilities|Time|GetWorldDeltaSeconds))))))
            (:NewEnumerator2
              (CallFunction|ConeRecoil))))
        (:3
          ;[1 1 1] Grenade Thrown
          (Animation|Montage|MontagePlay (Components|SkeletalMesh|GetAnimInstance (Variables|/Script/Engine.Character|GetMesh (Variables|MyCharacter|GetGunOwner))) "/Game/MyContent/Animations/Rifle/Aim/Rifle_Grenade_Throw_Far_Montage.Rifle_Grenade_Throw_Far_Montage" 1.0 "MontageLength" 0.0 true)
          (Game|SpawnActorfromClass "/Game/BallisticsVFX/FXSpawnerBlueprints/Projectiles/Grenade_Thrown.Grenade_Thrown_C" (Math|Transform|MakeTransform (.location _returnvalue_5) (.rotation _returnvalue_5) (.scale _returnvalue_5)) "AdjustIfPossibleButDontSpawnIfColliding" 0 true 25 0 :!pinned true) ; Spawn projectile
          (Audio|SpawnSoundAttached "/Game/BallisticsVFX/SFX/Whoosh/Whoosh_1_Cue.Whoosh_1_Cue" (Variables|Default|GetGrenadeSpawnPoint) "None" "0, 0, 0" "0, 0, 0" "KeepRelativeOffset" false 1.0 (Class|GameplayStatics|GetGlobalTimeDilation) 0.0 0 0))))))

(event Custom|TriggerReleasedEvent
  (bind (_aimtransform_location _returnvalue) (|ConeRecoilWorkout_3_2))
  (bind (_aimtransform_location_2 _returnvalue_2) (|ConeRecoilWorkout_3))
  (bind (_aimtransform_location_3 _returnvalue_3) (|ConeRecoilWorkout))
  (bind (_aimtransform_location_4 _returnvalue_4) (|ConeRecoilWorkout_2))
  (bind _gunowner (Variables|MyCharacter|GetGunOwner))
  (bind _aimtransform (Variables|AimOffset|GetAimTransform))
  (bind _gunowner_2 (Variables|MyCharacter|GetGunOwner))
  (bind _recoiltype (Variables|RecoilOptions|GetRecoilType))
  (bind _gunowner_3 (Variables|MyCharacter|GetGunOwner))
  (bind _gunowner_4 (Variables|MyCharacter|GetGunOwner))
  (bind _gunowner_5 (Variables|MyCharacter|GetGunOwner))
  (bind _recoiltype_2 (Variables|RecoilOptions|GetRecoilType))
  (bind _aimtransform_2 (Variables|AimOffset|GetAimTransform))
  (bind _recoiltype_3 (Variables|RecoilOptions|GetRecoilType))
  (bind _aimtransform_3 (Variables|AimOffset|GetAimTransform))
  (bind _recoiltype_4 (Variables|RecoilOptions|GetRecoilType))
  (bind _aimtransform_4 (Variables|AimOffset|GetAimTransform))
  (bind _gunowner_6 (Variables|MyCharacter|GetGunOwner))
  (bind _returnvalue_5 (Utilities|Select :Index _recoiltype_2 :NewEnumerator0 _aimtransform_4 :NewEnumerator1 _aimtransform_4 :NewEnumerator2 (Math|Transform|MakeTransform _aimtransform_location _returnvalue "1,1,1")))
  (bind _returnvalue_6 (Utilities|Select :Index _recoiltype_3 :NewEnumerator0 _aimtransform_2 :NewEnumerator1 _aimtransform_2 :NewEnumerator2 (Math|Transform|MakeTransform _aimtransform_location_3 _returnvalue_3 "1,1,1")))
  (bind _returnvalue_7 (Utilities|Select :Index _recoiltype :NewEnumerator0 _aimtransform :NewEnumerator1 _aimtransform :NewEnumerator2 (Math|Transform|MakeTransform _aimtransform_location_2 _returnvalue_2 "1,1,1")))
  (bind _returnvalue_8 (Utilities|Select :Index _recoiltype_4 :NewEnumerator0 _aimtransform_3 :NewEnumerator1 _aimtransform_3 :NewEnumerator2 (Math|Transform|MakeTransform _aimtransform_location_4 _returnvalue_4 "1,1,1")))
  (bind _mesh (Variables|/Script/Engine.Character|GetMesh _gunowner))
  (bind _mesh_2 (Variables|/Script/Engine.Character|GetMesh _gunowner_3))
  (bind _mesh_3 (Variables|/Script/Engine.Character|GetMesh _gunowner_4))
  (bind _returnvalue_9 (Components|SkeletalMesh|GetAnimInstance _mesh))
  (bind _returnvalue_10 (Components|SkeletalMesh|GetAnimInstance _mesh_2))
  (bind _returnvalue_11 (Components|SkeletalMesh|GetAnimInstance _mesh_3))
  ;[1 1 1] Trigger Press
  (Variables|MyCharacter|SetTriggerPressed false)
  (CallFunction|StopNoise)
  (CallFunction|TriggerOFF)
  (|FireRateAndSpamClickRegulation (Utilities|Select :Index (Variables|MyCharacter|GetSelectedWeapon) :Option%200 (Variables|FireRate|GetRifle%20Fire%20Rate) :Option%201 (Variables|FireRate|GetPistol%20Fire%20Rate) :Option%202 (Variables|FireRate|GetHiPowered%20Fire%20Rate) :Option%203 (Variables|FireRate|GetThrowGrenadeRate))) ; enters at TriggerOFF
)

(event Custom|BulletTimeEvent
  ;[1 1 1] BulletTime
  (if (Variables|MyCharacter|GetSlowmo?)
    (Variables|MyCharacter|SetSlowmo? false)
    (Utilities|Time|SetGlobalTimeDilation 1.0)
    (else
      (Variables|MyCharacter|SetSlowmo? true)
      (Utilities|Time|SetGlobalTimeDilation 0.35))))

(event Custom|AimOffsetTrigger
  ;[1 1 1] Aim Offset
  (Utilities|AimOffsetTrace (Variables|Default|GetFP_Gun) (Variables|AimOffset|GetAimOffsetMaxRange) (Variables|Default|GetProjectileSpawnPoint)))

(event Custom|ConeRecoil
  (bind _recoilconepershotadd (Variables|ConeRecoil|GetRecoilConePerShotAdd))
  ;[1 1 1] Cone Recoil Simple Example
  (bind _recoilconefloat (Timeline|ConeRecoilFloat PlayFromStart)
    (:Update
      (Variables|ConeRecoil|SetRecoilFloatSet _recoilconefloat)
      (Variables|ConeRecoil|SetConeRecoilYaw (* (Math|Float|Clamp(Float) (+ _recoilconepershotadd (Variables|ConeRecoil|GetConeRecoilYaw)) 0.0 (Variables|ConeRecoil|GetConeRecoilYawMAX)) _recoilconefloat))
      (Variables|ConeRecoil|SetConeRecoilPitch (* (Math|Float|Clamp(Float) (+ _recoilconepershotadd (Variables|ConeRecoil|GetConeRecoilPitch)) 0.0 (Variables|ConeRecoil|GetConeRecoilPitch%20MAX)) _recoilconefloat)))))

(event Custom|FireGrenadeLauncherEvent
  (bind _gunowner (Variables|MyCharacter|GetGunOwner))
  ;[1 1 1] Play Fire Animation
  (Animation|Montage|MontagePlay (Components|SkeletalMesh|GetAnimInstance (Variables|/Script/Engine.Character|GetMesh (Variables|MyCharacter|GetGunOwner))) "/Game/MyContent/Animations/Rifle/Aim/Rifle_ShootGrenade_Montage.Rifle_ShootGrenade_Montage" 1.0 "MontageLength" 0.0 true)
  ;[1 1 1] Grenade Launcher
  (Game|SpawnActorfromClass "/Game/BallisticsVFX/FXSpawnerBlueprints/Projectiles/Grenade_launched.Grenade_launched_C" (Math|Transform|MakeTransform (Transformation|GetSocketLocation (Variables|Default|GetGrenadeSpawnPoint) "None") (Pawn|GetControlRotation (Variables|/Script/Engine.Actor|GetInstigator (Components|GetOwner)) :!class /Script/Engine.Pawn)) "AdjustIfPossibleButDontSpawnIfColliding" 0 true 0 :!pinned true) ; Spawn projectile
  (Audio|SpawnSoundAttached "/Game/BallisticsVFX/SFX/GrenLauncher/GrenadeLauncher_cue.GrenadeLauncher_cue" (Variables|Default|GetProjectileSpawnPoint) "None" "0, 0, 0" "0, 0, 0" "KeepRelativeOffset" false 1.0 (Class|GameplayStatics|GetGlobalTimeDilation) 0.0 0 0)
  (switch Utilities|FlowControl|Switch|SwitchonRecoilType (Variables|RecoilOptions|GetRecoilType)
    (:NewEnumerator1
      ;[1 1 1] Recoil Grenade Fire
      (bind _recoil_float (Timeline|Timeline_6 PlayFromStart)
        (:Update
          (Pawn|Input|AddControllerPitchInput _gunowner (* (* (* _recoil_float (Variables|CameraRecoil|GetGrenadeLauncher_Recoil)) (Math|Random|RandomFloatinRange 0.9 1.1)) (Variables|MyCharacter|GetBaseLookUpRate) (Utilities|Time|GetWorldDeltaSeconds)))
          (Pawn|Input|AddControllerYawInput _gunowner (* (* (* (* (* _recoil_float (Variables|CameraRecoil|GetGrenadeLauncher_Recoil)) (Math|Random|RandomFloatinRange 0.9 1.1)) (Variables|CameraRecoil|GetGrenade_sideways)) (Math|Random|RandomFloatinRange -1.0 1.0)) (Variables|MyCharacter|GetBaseTurnRate) (Utilities|Time|GetWorldDeltaSeconds))))))
    (:NewEnumerator2
      (CallFunction|ConeRecoil))))

(event Custom|TriggerOFF
  ;[0.2075 0.4327 1] Activate Muzzle Smoke FX once trigger is lifted (we don't want to spawn too many smoke FX during rapid fire)
  (Components|Activation|Activate (Variables|Default|GetMuzzle_Smoke_light) false))

(event Custom|RifleSelectEvent
  ;[1 1 1] Weapon Select
  ;;[1 1 1] Rifle
  (if (not (== (Variables|MyCharacter|GetSelectedWeapon) 0))
    (Variables|MyCharacter|SetSelectedWeapon 0)
    (Variables|Default|SetIsPistolEquipped? false)
    (Variables|Default|SetIsGrenadeEquipped? false)
    ;;[1 1 1] Notify the Animation BP of weapon change
    (bind _asplayer_character_anim_bp (Utilities|Casting|CastToPlayerCharacter_AnimBP (Components|SkeletalMesh|GetAnimInstance (Variables|/Script/Engine.Character|GetMesh (Variables|MyCharacter|GetGunOwner)))))
    (Variables|/Game/MyContent/Blueprints/Characters/PlayerCharacter_AnimBP.PlayerCharacter_AnimBP_C|SetIsPistolEquipped? _asplayer_character_anim_bp false)))

(event Custom|TriggerON
  ;[0.2075 0.4327 1] Activate Muzzle Smoke FX once trigger is lifted (we don't want to spawn too many smoke FX during rapid fire)
  (CallFunction|MuzzleSmokeOff))

(event Custom|PistolSelectEvent
  ;[1 1 1] Weapon Select
  ;;[1 1 1] Pistol
  (if (not (== (Variables|MyCharacter|GetSelectedWeapon) 1))
    (Variables|MyCharacter|SetSelectedWeapon 1)
    (Variables|Default|SetIsPistolEquipped? true)
    (Variables|Default|SetIsGrenadeEquipped? false)
    ;;[1 1 1] Notify the Animation BP of weapon change
    (bind _asplayer_character_anim_bp (Utilities|Casting|CastToPlayerCharacter_AnimBP (Components|SkeletalMesh|GetAnimInstance (Variables|/Script/Engine.Character|GetMesh (Variables|MyCharacter|GetGunOwner)))))
    (Variables|/Game/MyContent/Blueprints/Characters/PlayerCharacter_AnimBP.PlayerCharacter_AnimBP_C|SetIsPistolEquipped? _asplayer_character_anim_bp true)))

(event Custom|SelectHPRifleEvent
  ;[1 1 1] Weapon Select
  ;;[1 1 1] HP Rifle
  (if (not (== (Variables|MyCharacter|GetSelectedWeapon) 2))
    (Variables|MyCharacter|SetSelectedWeapon 2)
    (Variables|Default|SetIsPistolEquipped? false)
    (Variables|Default|SetIsGrenadeEquipped? false)
    ;;[1 1 1] Notify the Animation BP of weapon change
    (bind _asplayer_character_anim_bp (Utilities|Casting|CastToPlayerCharacter_AnimBP (Components|SkeletalMesh|GetAnimInstance (Variables|/Script/Engine.Character|GetMesh (Variables|MyCharacter|GetGunOwner)))))
    (Variables|/Game/MyContent/Blueprints/Characters/PlayerCharacter_AnimBP.PlayerCharacter_AnimBP_C|SetIsPistolEquipped? _asplayer_character_anim_bp false)))

(event Custom|SelectGrenadeEvent
  ;[1 1 1] Weapon Select
  ;;[1 1 1] Grenade
  (if (not (== (Variables|MyCharacter|GetSelectedWeapon) 3))
    (Variables|MyCharacter|SetSelectedWeapon 3)
    (Variables|Default|SetIsPistolEquipped? false)
    (Variables|Default|SetIsGrenadeEquipped? true)
    ;;[1 1 1] Notify the Animation BP of weapon change
    (bind _asplayer_character_anim_bp (Utilities|Casting|CastToPlayerCharacter_AnimBP (Components|SkeletalMesh|GetAnimInstance (Variables|/Script/Engine.Character|GetMesh (Variables|MyCharacter|GetGunOwner)))))
    (Variables|/Game/MyContent/Blueprints/Characters/PlayerCharacter_AnimBP.PlayerCharacter_AnimBP_C|SetIsPistolEquipped? _asplayer_character_anim_bp false)
    (Variables|/Game/MyContent/Blueprints/Characters/PlayerCharacter_AnimBP.PlayerCharacter_AnimBP_C|SetIsGrenadeEquipped? _asplayer_character_anim_bp true)))

(event Custom|AimEvent
  ;[1 1 1] Aiming Mode
  (if (Variables|MyCharacter|GetAiming)
    (Variables|MyCharacter|SetAimingTransition true)
    (Utilities|FlowControl|Sequence
      (:then_0
        (Components|MoveComponentTo 0 "-0.000032,-0.000121,-156.681732" "0,-10.000000, 0" true true 0.2 false)
        (Variables|MyCharacter|SetAimingTransition false)
        (Variables|MyCharacter|SetAiming false))
      (:then_1
        (bind _range (Timeline|Timeline_4 ReverseFromEnd)
          (:Update
            (Variables|/Script/Engine.CameraComponent|SetFieldOfView (Variables|/Game/MyContent/Blueprints/Characters/MyPlayerCharacter.MyPlayerCharacter_C|GetHeadCamera (Variables|MyCharacter|GetGunOwner)) _range)))))
    (else
      (Variables|MyCharacter|SetAimingTransition true)
      (Utilities|FlowControl|Sequence
        (:then_0
          (Components|MoveComponentTo 0 "-6.396840,-8.680000,-153.756317" "0,-9.000000, 0" true true 0.2 false)
          (Variables|MyCharacter|SetAimingTransition false)
          (Variables|MyCharacter|SetAiming true))
        (:then_1
          (Timeline|Timeline_4 PlayFromStart))))))

(event Custom|ZoomTogglerEvent
  (bind _gunowner (Variables|MyCharacter|GetGunOwner))
  (bind _headcamera (Variables|/Game/MyContent/Blueprints/Characters/MyPlayerCharacter.MyPlayerCharacter_C|GetHeadCamera _gunowner))
  ;[1 1 1] Zoom Toggler
  (if (== (Variables|/Script/Engine.CameraComponent|GetFieldOfView (Variables|/Game/MyContent/Blueprints/Characters/MyPlayerCharacter.MyPlayerCharacter_C|GetHeadCamera (Variables|MyCharacter|GetGunOwner))) 75.0)
    (Variables|/Script/Engine.CameraComponent|SetFieldOfView _headcamera 4e+01)
    (Variables|MyCharacter|SetScopeActive true)
    (elif (== (Variables|/Script/Engine.CameraComponent|GetFieldOfView (Variables|/Game/MyContent/Blueprints/Characters/MyPlayerCharacter.MyPlayerCharacter_C|GetHeadCamera (Variables|MyCharacter|GetGunOwner))) 4e+01)
      (Variables|/Script/Engine.CameraComponent|SetFieldOfView _headcamera 1e+01)
      (Variables|MyCharacter|SetScopeActive true)
      (elif (== (Variables|/Script/Engine.CameraComponent|GetFieldOfView (Variables|/Game/MyContent/Blueprints/Characters/MyPlayerCharacter.MyPlayerCharacter_C|GetHeadCamera (Variables|MyCharacter|GetGunOwner))) 1e+01)
        (Variables|/Script/Engine.CameraComponent|SetFieldOfView _headcamera 75.0)
        (Variables|MyCharacter|SetScopeActive false)))))

(event Custom|GunAudioToggleEvent
  ;[1 1 1] Gun Audio Toggle
  (Utilities|FlowControl|FlipFlop
    (:A
      (Variables|MyCharacter|SetGunAudioToggle false))
    (:B
      (Variables|MyCharacter|SetGunAudioToggle true))))

(event Custom|MuzzleSmokeOff
  ;[0.2075 0.4327 1] MUZZLE SMOKE OFF
  (Components|Activation|Deactivate (Variables|Default|GetMuzzle_Smoke_light)))

(event Input|KeyboardEvents|C
  (params (Key :type Key%20Structure :default "None"))
  ;[1 1 1] Zoom Toggler
)

(event Input|KeyboardEvents|E
  (params (Key :type Key%20Structure :default "None"))
  ;[1 1 1] BulletTime
)