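; EnemyNPC is an AI enemy character that can take cover, take damage and be killed by player takedowns.
; Cover events toggle crouch, with leaving restarting the NPC behavior tree, while damage goes to a health component.
; Threatened raises a blackboard flag for five seconds, and an overlap area enables the player's takedown ahead of the victim's montage-and-destroy sequence.
; Its own trace-based takedown is partly disconnected, and attack, reload and bite events are empty.
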(event EventBeginPlay
  ;[1 1 1] Reference Owner's Animation BP
  (bind _asenemy_npc_anim_bp (Utilities|Casting|CastToEnemyNPC_AnimBP (Components|SkeletalMesh|GetAnimInstance (Variables|Character|GetMesh))))
  (Variables|Character|SetAnimInstanceRef _asenemy_npc_anim_bp))

(fn ConstructionScript)

(event Custom|LeaveCoverEvent
  (Variables|Cover|SetIsInCover? false)
  (Character|UnCrouch)
  (AI|RunBehaviorTree (AI|GetAIController self) "/Game/MyContent/AI/NPC_BT.NPC_BT"))

(event Custom|EnterCoverEvent
  (Variables|Cover|SetIsInCover? true)
  (Character|Crouch))

(event OnComponentHit(CapsuleComponent)
  (params (HitComponent :type Primitive%20Component%20Object%20Reference) (OtherActor :type Actor%20Object%20Reference) (OtherComp :type Primitive%20Component%20Object%20Reference) (NormalImpulse :type Vector :default "0, 0, 0") (Hit :type Hit%20Result%20Structure%20%28by%20ref%29)))

(event Game|Damage|EventAnyDamage
  (params (Damage :type Float%20%28single-precision%29) (DamageType :type Damage%20Type%20Object%20Reference) (InstigatedBy :type Controller%20Object%20Reference) (DamageCauser :type Actor%20Object%20Reference))
  (Default|CallRecieveDamage (Variables|Default|GetHealth_CBP) Damage))

(event Collision|EventHit
  (params (MyComp :type Primitive%20Component%20Object%20Reference) (Other :type Actor%20Object%20Reference) (OtherComp :type Primitive%20Component%20Object%20Reference) (bSelfMoved :type Boolean) (HitLocation :type Vector :default "0, 0, 0") (HitNormal :type Vector :default "0, 0, 0") (NormalImpulse :type Vector :default "0, 0, 0") (Hit :type Hit%20Result%20Structure%20%28by%20ref%29)))

(event Game|Damage|EventPointDamage
  (params (Damage :type Float%20%28single-precision%29) (DamageType :type Damage%20Type%20Object%20Reference) (HitLocation :type Vector :default "0, 0, 0") (HitNormal :type Vector :default "0, 0, 0") (HitComponent :type Primitive%20Component%20Object%20Reference) (BoneName :type Name :default "None") (ShotFromDirection :type Vector :default "0, 0, 0") (InstigatedBy :type Controller%20Object%20Reference) (DamageCauser :type Actor%20Object%20Reference) (HitInfo :type Hit%20Result%20Structure%20%28by%20ref%29)))

(event Game|Damage|EventRadialDamage
  (params (DamageReceived :type Float%20%28single-precision%29) (DamageType :type Damage%20Type%20Object%20Reference) (Origin :type Vector :default "0, 0, 0") (HitInfo :type Hit%20Result%20Structure%20%28by%20ref%29) (InstigatedBy :type Controller%20Object%20Reference) (DamageCauser :type Actor%20Object%20Reference)))

(event Custom|AttackEvent
  ;[1 1 1] Attack
)

(event Custom|Threatened
  ;[1 1 1] Threatened
  (Variables|Threat|SetIsThreatened? true)
  (AI|Components|Blackboard|SetValueasBool (AI|GetBlackboard 0) (Utilities|Name|MakeLiteralName "IsThreatened?") (Variables|Threat|GetIsThreatened?))
  (Utilities|FlowControl|Delay 5.0)
  (Variables|Threat|SetIsThreatened? false)
  (AI|Components|Blackboard|SetValueasBool (AI|GetBlackboard 0) (Utilities|Name|MakeLiteralName "IsThreatened?") (Variables|Threat|GetIsThreatened?)))

(event Custom|ReloadEvent
  ;[1 1 1] Reload
)

(event Custom|BiteEvent
  ;[1 1 1] Reload
)

(event Custom|Attack%20Stop%20Event
  ;[1 1 1] Attack
)

(event OnComponentEndOverlap(TakedownArea)
  (params (OverlappedComponent :type Primitive%20Component%20Object%20Reference) (OtherActor :type Actor%20Object%20Reference) (OtherComp :type Primitive%20Component%20Object%20Reference) (OtherBodyIndex :type Integer))
  ;[1 1 1] Takedown
  (bind _asbfxcharacter_bp (Utilities|Casting|CastToBFXCharacter_BP OtherActor))
  (Variables|/Game/MyContent/Blueprints/Characters/BFXCharacter_BP.BFXCharacter_BP_C|SetCanTakedown? _asbfxcharacter_bp false))

(event OnComponentBeginOverlap(TakedownArea)
  (params (OverlappedComponent :type Primitive%20Component%20Object%20Reference) (OtherActor :type Actor%20Object%20Reference) (OtherComp :type Primitive%20Component%20Object%20Reference) (OtherBodyIndex :type Integer) (bFromSweep :type Boolean) (SweepResult :type Hit%20Result%20Structure%20%28by%20ref%29))
  ;[1 1 1] Takedown
  (bind _asbfxcharacter_bp (Utilities|Casting|CastToBFXCharacter_BP OtherActor))
  (Variables|/Game/MyContent/Blueprints/Characters/BFXCharacter_BP.BFXCharacter_BP_C|SetCanTakedown? _asbfxcharacter_bp true))

(event Custom|TakedownSequence
  ;[1 1 1] Takedown
  (Pawn|Components|CharacterMovement|DisableMovement (Variables|Character|GetCharacterMovement))
  (Collision|SetActorEnableCollision false)
  (Animation|PlayAnimMontage 0 1.0 "None")
  (Utilities|FlowControl|Delay 1e+01)
  (Actor|DestroyActor))

(event Custom|TakedownEvent
  (bind _returnvalue (Transformation|GetActorLocation))
  ;[1 1 1] Takedown
  (if (Variables|Takedown|GetCanTakeDown?)
    (bind (_outhit _returnvalue_2) (Collision|LineTraceByChannel _returnvalue (+ _returnvalue (* (Transformation|GetActorForwardVector) 2.5e+02)) "TraceTypeQuery1" false 0 "None"))
    (if _returnvalue_2
      (bind _asbfxcharacter_bp (Utilities|Casting|CastToBFXCharacter_BP (.HitActor (Collision|BreakHitResult _outhit))))
      (Variables|Takedown|SetTakedownTarget _asbfxcharacter_bp)
      (Transformation|AttachComponentToComponent (Variables|Default|GetCameraBoom) (Variables|Character|GetMesh) "spine_02" "SnapToTarget" "SnapToTarget" "SnapToTarget" true)
      (Pawn|Components|CharacterMovement|DisableMovement (Variables|Character|GetCharacterMovement))
      (Variables|Takedown|SetCanTakeDown? false)
      (Transformation|SetActorTransform (Math|Transform|MakeTransform (+ (.location (Transformation|GetActorTransform (Variables|Takedown|GetTakedownTarget))) (* (Transformation|GetActorForwardVector (Variables|Takedown|GetTakedownTarget)) -175.0)) (.rotation (Transformation|GetActorTransform (Variables|Takedown|GetTakedownTarget))) "1,1,1"))
      (bind _returnvalue_3 (Animation|PlayAnimMontage 0 1.0 "None")))))

(event Input|ActionEvents|InputActionTakedown
  (params (Key :type Key%20Structure))
  (bind _returnvalue (Transformation|GetActorLocation))
  ;[1 1 1] Takedown
  (:Pressed
    (if (Variables|Takedown|GetCanTakeDown?)
      (bind (_outhit _returnvalue_2) (Collision|LineTraceByChannel _returnvalue (+ _returnvalue (* (Transformation|GetActorForwardVector) 2.5e+02)) "TraceTypeQuery1" false 0 "None"))
      (if _returnvalue_2
        (bind _asbfxcharacter_bp (Utilities|Casting|CastToBFXCharacter_BP (.HitActor (Collision|BreakHitResult _outhit))))
        (Variables|Takedown|SetTakedownTarget _asbfxcharacter_bp)
        (Transformation|AttachComponentToComponent (Variables|Default|GetCameraBoom) (Variables|Character|GetMesh) "spine_02" "SnapToTarget" "SnapToTarget" "SnapToTarget" true)
        (Pawn|Components|CharacterMovement|DisableMovement (Variables|Character|GetCharacterMovement))
        (Variables|Takedown|SetCanTakeDown? false)
        (Transformation|SetActorTransform (Math|Transform|MakeTransform (+ (.location (Transformation|GetActorTransform (Variables|Takedown|GetTakedownTarget))) (* (Transformation|GetActorForwardVector (Variables|Takedown|GetTakedownTarget)) -175.0)) (.rotation (Transformation|GetActorTransform (Variables|Takedown|GetTakedownTarget))) "1,1,1"))
        (bind _returnvalue_3 (Animation|PlayAnimMontage 0 1.0 "None"))))))