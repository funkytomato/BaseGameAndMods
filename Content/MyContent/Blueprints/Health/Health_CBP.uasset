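; Health component that tracks a character's health and armour, along with dead and no-armour flags.
; On BeginPlay it binds handlers for damage, health boost and armour boost events.
; Damage drains armour first, and any hit that leaves armour at zero also deals its full amount to health.
; Health changes trigger an update for the blood screen, while the armour boost handler is empty, leaving IncreaseArmour unused.
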(event Custom|RecieveDamage_Event
  (params (damageAmount :type Float%20%28single-precision%29))
  ;[1 1 1] Recieved Damage Event Dispatcher
  ;;[1 1 1] Reduce Armour before Health
  (CallFunction|DecreaseArmour damageAmount)
  (if (Variables|Default|GetnoArmour?)
    (bind _currenthealth (CallFunction|DecreaseHealth damageAmount))
    ;;[1 1 1] Update Blood Screen
    (Default|CallUpdateHealth _currenthealth)))

(event Custom|HealthBoost_Event
  (params (healthBoost :type Float%20%28single-precision%29))
  ;[1 1 1] Increase Boost Event Dispatcher
  ;;[1 1 1] Increase Health
  (bind _currenthealth (CallFunction|IncreaseHealth healthBoost))
  ;;[1 1 1] Update Blood Screen
  (Default|CallUpdateHealth _currenthealth))

(event Custom|ArmorBoost_Event
  (params (boostAmount :type Float%20%28single-precision%29)))

(event EventBeginPlay
  ;[1 1 1] Recieved Damage Event Dispatcher
  (EventDispatchers|BindEventtoRecieveDamage (delegate Custom|RecieveDamage_Event))
  ;[1 1 1] Increase Boost Event Dispatcher
  (EventDispatchers|BindEventtoHealthBoost (delegate Custom|HealthBoost_Event))
  (EventDispatchers|BindEventtoArmorBoost (delegate Custom|ArmorBoost_Event)))

(fn IncreaseHealth
  (params (value :type Float%20%28single-precision%29))
  (bind _output_get (Variables|Default|SetHealth (Math|Float|Clamp(Float) (+ (Variables|Default|GetHealth) value) 0.0 (Variables|Default|GetMaxHealth))))
  (Variables|Default|SetIsDead? (not (> _output_get 0.0)))
  (return _output_get))

(fn DecreaseHealth
  (params (value :type Float%20%28single-precision%29))
  (bind _output_get (Variables|Default|SetHealth (Math|Float|Clamp(Float) (- (Variables|Default|GetHealth) value) 0.0 (Variables|Default|GetMaxHealth))))
  (Variables|Default|SetIsDead? (not (> _output_get 0.0)))
  (return _output_get))

(fn DecreaseArmour
  (params (amount :type Float%20%28single-precision%29))
  (bind _output_get (Variables|Default|SetArmour (Math|Float|Clamp(Float) (- (Variables|Default|GetArmour) amount) 0.0 (Variables|Default|GetMaxArmour))))
  (Variables|Default|SetnoArmour? (== _output_get 0.0)))

(fn IncreaseArmour
  (params (amount :type Float%20%28single-precision%29))
  (bind _output_get (Variables|Default|SetArmour (Math|Float|Clamp(Float) (+ (Variables|Default|GetArmour) amount) 0.0 (Variables|Default|GetMaxArmour))))
  (Variables|Default|SetnoArmour? (not (> _output_get 0.0))))