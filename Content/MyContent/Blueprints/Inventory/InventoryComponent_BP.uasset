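; Inventory component that stores item entries and toggles the inventory screen.
; InventoryEvent uses a FlipFlop to pause and show the inventory widget with the mouse cursor, then unpause, remove it and create a new player HUD; the HUD-removal nodes are unconnected.
; AddItemToInventory loops over existing entries, appending a summed-quantity copy on a name match or add-unique otherwise, so an empty inventory receives nothing.
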(event Custom|InventoryEvent
  (bind _returnvalue (Game|GetPlayerController 0))
  (Utilities|FlowControl|FlipFlop
    (:A
      (Game|SetGamePaused (Variables|Default|GetPaused))
      (bind _returnvalue_2 (UserInterface|CreateWidget "/Game/MyContent/Blueprints/Inventory/InventorySystem_WBP.InventorySystem_WBP_C" (Game|GetPlayerController 0)))
      (UserInterface|Viewport|AddtoViewport _returnvalue_2 0)
      (Variables|/Script/Engine.PlayerController|SetbShowMouseCursor _returnvalue true))
    (:B
      (Game|SetGamePaused (Variables|Default|GetUnPaused))
      (Widget|RemovefromParent _returnvalue_2)
      (Variables|/Script/Engine.PlayerController|SetbShowMouseCursor _returnvalue false)
      (bind _returnvalue_3 (UserInterface|CreateWidget "/Game/MyContent/UI/PlayerHUD_WBP.PlayerHUD_WBP_C" (Game|GetPlayerController 0)))
      (UserInterface|Viewport|AddtoViewport _returnvalue_3 0))))

(fn AddItemtoInventory
  (params (itemToAdd :type Inventory%20Item%20Struct%20Structure))
  (bind (_itemname _itemqty) (Utilities|Struct|BreakInventoryItemStruct itemToAdd))
  (Development|PrintString (Utilities|String|ToString(Integer) (Utilities|Array|Length (Variables|Default|GetInventory))))
  (bind _array_element (Utilities|Array|ForEachLoopwithBreak (Variables|Default|GetInventory) :!label _label)
    (:LoopBody
      (if (Utilities|Enum|Equal(Enum) (.ItemName (Utilities|Struct|BreakInventoryItemStruct _array_element)) _itemname)
        (bind _output_get (LocalVariables|SetitemChanged (Utilities|Struct|MakeInventoryItemStruct (.ItemName (Utilities|Struct|BreakInventoryItemStruct _array_element)) (+ (.ItemQty (Utilities|Struct|BreakInventoryItemStruct _array_element)) _itemqty) (.ItemImage (Utilities|Struct|BreakInventoryItemStruct _array_element)))))
        (Utilities|Array|Add (Variables|Default|GetInventory) _output_get)
        (goto _label Break)
        (else
          (Utilities|Array|AddUnique (Variables|Default|GetInventory) itemToAdd))))
    (:Completed
      (Development|PrintString "Item has been add to inventory")
      (Development|PrintString (Utilities|String|ToString(Integer) (Utilities|Array|Length (Variables|Default|GetInventory)))))))