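; Actor component that gives MyPlayerCharacter partial-ragdoll hit reactions through a PhysicalAnimation component it adds at BeginPlay.
; HitReaction simulates bodies below the pelvis and applies an impulse along the trace to the hit bone, redirecting pelvis hits to spine_01.
; Tick decays an accumulating timer that drives physics blend weight, then stops simulation and disables itself.
; A separate flip-flop event toggles half-blended physics below the pelvis.
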(event Custom|TogglePhysicalAnimation
  (bind _physicalanimcomp (Variables|Default|GetPhysicalAnimComp))
  (Utilities|FlowControl|FlipFlop
    (:A
      (Collision|SetActorEnableCollision (Variables|Default|GetMyCharacter) true)
      (Class|SkeletalMeshComponent|SetAllBodiesBelowSimulatePhysics (Variables|Default|GetMesh) (Utilities|Name|MakeLiteralName "Pelvis") true false)
      (Class|PhysicalAnimationComponent|ApplyPhysicalAnimationProfileBelow _physicalanimcomp "Pelvis" "HitReactionProfile" false false)
      (Class|PhysicalAnimationComponent|SetStrengthMultiplyer _physicalanimcomp 0.0)
      (Class|SkeletalMeshComponent|SetAllBodiesBelowPhysicsBlendWeight (Variables|Default|GetMesh) (Utilities|Name|MakeLiteralName "Pelvis") 0.5 false true))
    (:B
      (Class|SkeletalMeshComponent|SetAllBodiesBelowSimulatePhysics (Variables|Default|GetMesh) (Utilities|Name|MakeLiteralName "Pelvis") false false))))

(event Custom|HitReaction
  (params (Hit :type Hit%20Result%20Structure))
  (bind (_bblockinghit _binitialoverlap _time _distance _location _impactpoint _normal _impactnormal _physmat _hitactor _hitcomponent _hitbonename _hititem _elementindex _faceindex _tracestart _traceend) (Collision|BreakHitResult Hit))
  (Components|Tick|SetComponentTickEnabled true)
  (Variables|Default|SetHitReactionTimeRemaining (+ (Variables|Default|GetHitReactionTimeRemaining) 2.0))
  (Class|PhysicalAnimationComponent|ApplyPhysicalAnimationProfileBelow (Variables|Default|GetPhysicalAnimComp) "pelvis" "HitReactionProfile" false false)
  (Class|SkeletalMeshComponent|SetAllBodiesBelowSimulatePhysics (Variables|Default|GetMesh) (Utilities|Name|MakeLiteralName "Pelvis") true false)
  (Physics|AddImpulse (Variables|Default|GetMesh) (* (Math|Vector|Normalize (- _traceend _tracestart)) 5e+03) (select (Utilities|Name|Equal(Name) _hitbonename "pelvis") (Utilities|Name|MakeLiteralName "spine_01") _hitbonename) true))

(event EventBeginPlay
  (bind _returnvalue (Components|GetOwner))
  (bind _returnvalue_2 (Game|AddComponentbyClass _returnvalue "/Script/Engine.PhysicalAnimationComponent"))
  (bind _output_get (Variables|Default|SetPhysicalAnimComp _returnvalue_2))
  (bind _asmy_player_character (Utilities|Casting|CastToMyPlayerCharacter _returnvalue))
  (Variables|Default|SetMyCharacter _asmy_player_character)
  (Variables|Default|SetMesh (Variables|/Script/Engine.Character|GetMesh _asmy_player_character))
  (Class|PhysicalAnimationComponent|SetSkeletalMeshComponent _output_get (Variables|/Script/Engine.Character|GetMesh _asmy_player_character)))

(event EventTick
  (params (DeltaSeconds :type Float%20%28single-precision%29))
  (Variables|Default|SetHitReactionTimeRemaining (- (Math|Interpolation|FInterpTo (Variables|Default|GetHitReactionTimeRemaining) 0.0 0.0 1.0) (* DeltaSeconds 0.1)))
  (if (<= (Variables|Default|GetHitReactionTimeRemaining) 0.0)
    (Variables|Default|SetHitReactionTimeRemaining 0.0)
    (Class|SkeletalMeshComponent|SetAllBodiesBelowSimulatePhysics (Variables|Default|GetMesh) (Utilities|Name|MakeLiteralName "pelvis") false true)
    (Components|Tick|SetComponentTickEnabled false)
    (else
      (Class|SkeletalMeshComponent|SetAllBodiesBelowPhysicsBlendWeight (Variables|Default|GetMesh) (Utilities|Name|MakeLiteralName "pelvis") (Math|Float|Min(Float) (Variables|Default|GetHitReactionTimeRemaining) 1.0) false true))))